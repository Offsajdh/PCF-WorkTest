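; MainCharacter_BP is the player character for what appears to be an auto-runner, moving constantly along world +X at RunSpeed every Tick.
; A Move Right / Left axis strafes it along the control rotation's right vector.
; The Jump action triggers the built-in jump and holds a Jumping flag true for a short fixed delay rather than until landing.
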(event `self.ReceiveTick`
  (params (DeltaSeconds :type "Float (single-precision)"))
  (`self.AddMovementInput` (1.0 0.0 0.0) (`self.RunSpeed`)))

(event `InputAction|Jump`
  (params (Key :type "Key Structure"))
  (:`Pressed`
    (`self.Jump`)
    (set `self.Jumping` true)
    (`KismetSystemLibrary.Delay` 0.8)
    (set `self.Jumping` false)))

(event `InputAxis|Move Right / Left`
  (params (AxisValue :type "Float (single-precision)"))
  (`self.AddMovementInput` (`KismetMathLibrary.GetRightVector` (`self.GetControlRotation`)) AxisValue))

(fn `UserConstructionScript`)